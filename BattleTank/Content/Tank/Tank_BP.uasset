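; Player-controllable tank Blueprint that sets up aiming references, orbit camera controls and firing.
; On BeginPlay it passes its Barrel and Turret components to setter functions defined outside these graphs.
; Azimuth input yaws a gimbal and elevation input pitches the spring arm, keeping the two camera rotations on separate components.
; Left mouse press calls Fire, whose logic also lives outside these graphs.
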(event `self.ReceiveBeginPlay`
  (`self.SetBarrelReference` (`self.Barrel`))
  (`self.SetTurretReference` (`self.Turret`)))

(event `InputAxis|AimAzimuth`
  (params (AxisValue :type "Float (single-precision)"))
  ;[1 1 1] Camera Input Binding
  (`SceneComponent.K2_AddLocalRotation` (`self.AzimuthGimbal`) (`KismetMathLibrary.MakeRotator` 0.0 0.0 AxisValue) false false))

(event `InputAxis|AimElevation`
  (params (AxisValue :type "Float (single-precision)"))
  ;[1 1 1] Camera Input Binding
  (`SceneComponent.K2_AddLocalRotation` (`self.SpringArm`) (`KismetMathLibrary.MakeRotator` 0.0 AxisValue) false false))

(event `Key|LeftMouseButton`
  (params (Key :type "Key Structure"))
  ;[1 1 1] Camera Input Binding
  (:`Pressed`
    (`self.Fire`)))

(fn `UserConstructionScript`)